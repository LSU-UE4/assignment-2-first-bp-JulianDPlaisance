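; Guess-number mini-game Blueprint where Space steps a counter until it matches a target number that is shown on screen.
; Each press updates the ReadyPlayerOne text, wrapping to zero once the count passes 20.
; BeginPlay and Tick share a comparison that shows either the target or victory text in Rando.
; A match waits through a short Delay, then rolls a new random target and resets the counter.
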(event EventTick
  (params (DeltaSeconds :type Float%20%28single-precision%29))
  (bind _rando (Variables|Default|GetRando))
  ;[1 1 1] Every Tick, check to see if Rand && MyVar are ==
  (if (== (Variables|Default|GetMyVar) (Variables|Default|GetRand))
    ;[1 1 1] Reseting the Game to a new Random Integer and MyVar to 0
    (Rendering|Components|TextRender|SetText _rando (Variables|Default|GetVictoryText?))
    (Utilities|FlowControl|Delay 2.0)
    (Variables|Default|SetRand (Math|Random|RandomIntegerinRange 1 20))
    (Variables|Default|SetMyVar 0)
    ;[1 1 1] Incrementing Player's Guess(?) when they press space unless they pass 20 in which case it resets it to 0
    (Rendering|Components|TextRender|SetText (Variables|Default|GetReadyPlayerOne) (Utilities|Text|ToText(Integer) (stale Input|KeyboardEvents|SpaceBar _output_get)))
    (else
      ;[1 1 1] If MyVar is not equal to Rand then set Rando text to Rand
      (Rendering|Components|TextRender|SetText _rando (Utilities|Text|ToText(Integer) (Variables|Default|GetRand))))))

(event EventBeginPlay
  (bind _rando (Variables|Default|GetRando))
  ;[1 1 1] Every Tick, check to see if Rand && MyVar are ==
  (if (== (Variables|Default|GetMyVar) (Variables|Default|GetRand))
    ;[1 1 1] Reseting the Game to a new Random Integer and MyVar to 0
    (Rendering|Components|TextRender|SetText _rando (Variables|Default|GetVictoryText?))
    (Utilities|FlowControl|Delay 2.0)
    (Variables|Default|SetRand (Math|Random|RandomIntegerinRange 1 20))
    (Variables|Default|SetMyVar 0)
    ;[1 1 1] Incrementing Player's Guess(?) when they press space unless they pass 20 in which case it resets it to 0
    (Rendering|Components|TextRender|SetText (Variables|Default|GetReadyPlayerOne) (Utilities|Text|ToText(Integer) (stale Input|KeyboardEvents|SpaceBar _output_get)))
    (else
      ;[1 1 1] If MyVar is not equal to Rand then set Rando text to Rand
      (Rendering|Components|TextRender|SetText _rando (Utilities|Text|ToText(Integer) (Variables|Default|GetRand))))))

(event Input|KeyboardEvents|SpaceBar
  (params (Key :type Key%20Structure))
  ;[1 1 1] Incrementing Player's Guess(?) when they press space unless they pass 20 in which case it resets it to 0
  (:Pressed
    (bind _result (Math|Integer|IncrementInt (Variables|Default|GetMyVar))
      (:%20%20
        (bind _output_get (Variables|Default|SetMyVar _result))
        (if (> _output_get 20)
          (Variables|Default|SetMyVar 0))
        (Rendering|Components|TextRender|SetText (Variables|Default|GetReadyPlayerOne) (Utilities|Text|ToText(Integer) _output_get))))))

(fn ConstructionScript)